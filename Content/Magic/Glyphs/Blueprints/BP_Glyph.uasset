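; Base glyph actor for the magic system, representing one glyph within a cast spell.
; Cast stores the spell, index, cast glyphs and player, then attaches an optional Niagara effect to the root and binds termination handlers.
; Terminate broadcasts OnTerminate only once, whether called directly or triggered by destruction.
; HandleTerminate and GetPhysicalRepresentation are empty stubs, apparently meant for child glyphs to override.
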(event `Cast`
  (params (Spell :type "/Game/Magic/S_Spell Structure") (Index :type Integer) (CastGlyphs :type "Array of /Game/Magic/Glyphs/Blueprints/BP_Glyph Object Reference") (Player :type "/Game/Player/Blueprints/BP_Player Object Reference"))
  (bind _returnvalue (`SceneComponent.K2_GetComponentLocation` (`self.DefaultSceneRoot`)))
  (set `self.Spell` Spell)
  (set `self.Index` Index)
  (set `self.Player` Player)
  (set `self.Cast Glyphs` CastGlyphs)
  (`|ExecutionSequence`
    (:`then_0`
      (`/Engine/EditorBlueprintResources/StandardMacros.IsValid` (`self.ParticleTemplate`)
        (:`Is Valid`
          (bind _returnvalue_2 (`NiagaraFunctionLibrary.SpawnSystemAttached` (`self.ParticleTemplate`) (`self.DefaultSceneRoot`) "None" _returnvalue (struct) "SnapToTarget"))
          (bind _output_get (set `self.Particles` _returnvalue_2))
          (`SceneComponent.K2_SetWorldLocation` _output_get _returnvalue false false))))
    (:`then_1`
      (add `self.OnTerminate` (delegate `HandleTerminate`))
      (add `self.OnDestroyed` (delegate `TerminateOnDestroy`)))))

(event `HandleTerminate`)

(event `TerminateOnDestroy` :!signature `self.OnDestroyed`
  (params (DestroyedActor :type "Actor Object Reference"))
  (`self.Terminate`))

(event `Terminate`
  (`/Engine/EditorBlueprintResources/StandardMacros.DoOnce` false
    (:`Completed`
      (`self.OnTerminate`))))

(fn `GetPhysicalRepresentation`
  (returns (`Physical Components` :type "Array of PrimitiveComponent Object Reference"))
  (return))

(fn `UserConstructionScript`)